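; Vive tracker performer rig that drives neck and hand components from Live Link, with particle wings and sparks.
; Each tick applies scaling and the neck's calibration offset to all three positions, captured after BeginPlay or on R.
; Wings rotate along neck-to-hand directions and receive those distances as particle parameters.
; Keys 4/5 adjust particle spawn rate and spacing, 0 toggles a blackout fade, and the ground check is disconnected.
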(event `self.ReceiveTick`
  (params (DeltaSeconds :type "Float (single-precision)"))
  (`self.Debug Lines`)
  (bind _dataresult (`|EvaluateLiveLinkFrameWithSpecificRole` (struct :`Name` "/user/vive_tracker_htcx/role/left_elbow") "/Script/LiveLinkInterface.LiveLinkTransformRole") ; Track Neck
    (:`then`
      (`SceneComponent.K2_SetRelativeTransform` (`self.Neck`) (`KismetMathLibrary.MakeTransform` (* (+ (.location (`.Transform` (break `LiveLinkTransformFrameData` (`.FrameData` (break `LiveLinkTransformBlueprintData` _dataresult))))) (`|GetArrayItem` (`self.Offset`))) (`self.Scaling`))) false false)
      (bind _dataresult_2 (`|EvaluateLiveLinkFrameWithSpecificRole` (struct :`Name` "/user/vive_tracker_htcx/role/camera") "/Script/LiveLinkInterface.LiveLinkTransformRole") ; Track Right Hand
        (:`then`
          (`SceneComponent.K2_SetRelativeTransform` (`self.RightHand`) (`KismetMathLibrary.MakeTransform` (* (+ (.location (`.Transform` (break `LiveLinkTransformFrameData` (`.FrameData` (break `LiveLinkTransformBlueprintData` _dataresult_2))))) (`|GetArrayItem` (`self.Offset`))) (`self.Scaling`))) false false)
          (bind _dataresult_3 (`|EvaluateLiveLinkFrameWithSpecificRole` (struct :`Name` "/user/vive_tracker_htcx/role/chest") "/Script/LiveLinkInterface.LiveLinkTransformRole") ; Track Left Hand
            (:`then`
              (`SceneComponent.K2_SetRelativeTransform` (`self.LeftHand`) (`KismetMathLibrary.MakeTransform` (* (+ (.location (`.Transform` (break `LiveLinkTransformFrameData` (`.FrameData` (break `LiveLinkTransformBlueprintData` _dataresult_3))))) (`|GetArrayItem` (`self.Offset`))) (`self.Scaling`))) false false))))))))

(event `self.ReceiveBeginPlay`
  (bind (_returnvalue_x _returnvalue_y _returnvalue_z) (`KismetMathLibrary.BreakVector` (`SceneComponent.K2_GetComponentLocation` (`self.DefaultSceneRoot`))))
  (`|ExecutionSequence`
    (:`then_0`
      (`self.EnableInput` (`GameplayStatics.GetPlayerController` 0))
      (set `self.StartingHeight` _returnvalue_z))
    (:`then_1`
      (`KismetSystemLibrary.Delay` 0.2)
      (`self.Calibrate`))
    (:`then_2`
      (bind _returnvalue (`|CreateWidget` "/Game/BrianFolder/W_Blackout.W_Blackout_C"))
      (set `self.BlackoutWidget` _returnvalue)
      (`UserWidget.AddToViewport` _returnvalue 0))
    (:`then_3`
      (`self.set span rate`))))

(event `Key|R`
  (params (Key :type "Key Structure"))
  (:`Pressed`
    (`self.Calibrate`)))

(event `Calibrate`
  ;[0 0.6201 1] Brian's calibration based on BF_Vivetracked
  (`KismetArrayLibrary.Array_Set` (`self.Offset`) 0 (* (.location (`.Transform` (break `LiveLinkTransformFrameData` (`.FrameData` (break `LiveLinkTransformBlueprintData` (stale `self.ReceiveTick` _dataresult)))))) -1.0))
  (`KismetArrayLibrary.Array_Set` (`self.Offset`) 1 (* (.location (`.Transform` (break `LiveLinkTransformFrameData` (`.FrameData` (break `LiveLinkTransformBlueprintData` (stale `self.ReceiveTick` _dataresult_2)))))) -1.0))
  (`KismetArrayLibrary.Array_Set` (`self.Offset`) 2 (* (.location (`.Transform` (break `LiveLinkTransformFrameData` (`.FrameData` (break `LiveLinkTransformBlueprintData` (stale `self.ReceiveTick` _dataresult_3)))))) -1.0))
  (`KismetSystemLibrary.PrintString` "." true true (struct :`G` 0.066989 :`B` 1.0 :`A` 1.0) 1.0))

(event `Key|Zero`
  (params (Key :type "Key Structure"))
  (:`Pressed`
    (`self.FlipBlackLevels`)))

(event `FlipBlackLevels`
  ;[1 1 1] Comment
  (`/Engine/EditorBlueprintResources/StandardMacros.FlipFlop`
    (:`A`
      (bind (_direction _newtrack_0) (`Timeline|Timeline` :!via `PlayFromStart` :!label _label)
        (:`Update`
          (set `/Game/BrianFolder/W_Blackout.COlor` (make `LinearColor` 0.0 0.0 0.0 _newtrack_0) (`self.BlackoutWidget`)))
        (:`Finished`
          (`KismetSystemLibrary.PrintString` "Done"))))
    (:`B`
      (goto _label :!via `ReverseFromEnd`))))

(event `look  at hands`
  ;[0.1168 0.08209 1] Getting the Wings to point at the neck
  (`SceneComponent.K2_SetWorldRotation` (`self.Right Wing`) (`KismetMathLibrary.FindLookAtRotation` (`SceneComponent.K2_GetComponentLocation` (`self.Neck`)) (`SceneComponent.K2_GetComponentLocation` (`self.RightHand`))) false false)
  (`SceneComponent.K2_SetWorldRotation` (`self.Left Wing`) (`KismetMathLibrary.FindLookAtRotation` (`SceneComponent.K2_GetComponentLocation` (`self.Neck`)) (`SceneComponent.K2_GetComponentLocation` (`self.LeftHand`))) false false))

(event `Debug Lines`
  ;[1 1 1] Drawing Debug Lines
  (`|ExecutionSequence`
    (:`then_0`
      (`self.look  at hands`))
    (:`then_1`
      ;[0.4479 0 0.2144] Setting the length of the particle emitter equal to the distance between the neck and the hands
      (`NiagaraComponent.SetVariableFloat` (`self.Left Wing`) "float" (`KismetMathLibrary.Vector_Distance` (`SceneComponent.K2_GetComponentLocation` (`self.Neck`)) (`SceneComponent.K2_GetComponentLocation` (`self.LeftHand`)))) ; Set The Distance for the Left Hand to the Neck
      (`NiagaraComponent.SetVariableFloat` (`self.Right Wing`) "float" (`KismetMathLibrary.Vector_Distance` (`SceneComponent.K2_GetComponentLocation` (`self.Neck`)) (`SceneComponent.K2_GetComponentLocation` (`self.RightHand`)))) ; Set the Distance for the Right hand to the Neck
    )
    (:`then_2`
      (`self.VerticalCheck`))))

(event `VerticalCheck`
  ;[1 1 1] make sure the hands don't go in the ground.
)

(event `Key|Four`
  (params (Key :type "Key Structure"))
  (bind _spawn_spacing (`self.spawn spacing`))
  (bind _returnvalue (/ (`self.spawn rate`) 2.0))
  (bind _returnvalue_2 (/ (`self.spawn spacing`) 10.0))
  (:`Pressed`
    (`/Engine/EditorBlueprintResources/StandardMacros.CompareFloat` (`self.spawn rate`) 60.0
      (:`>`
        (set `self.spawn rate` (`KismetMathLibrary.FMax` (- (`self.spawn rate`) 10.0)))
        (set `self.spawn spacing` (* (`self.spawn spacing`) (`self.spacing multiplier`)))
        (`NiagaraComponent.SetVariableFloat` (`self.Right Sparks`) "SpawnRate" (`self.spawn rate`) :!label _label)
        (`NiagaraComponent.SetVariableFloat` (`self.Right Wing`) "SpawnRate" _returnvalue)
        (`NiagaraComponent.SetVariableFloat` (`self.Left Sparks`) "SpawnRate" (`self.spawn rate`))
        (`NiagaraComponent.SetVariableFloat` (`self.Left Wing`) "SpawnRate" _returnvalue)
        (`NiagaraComponent.SetVariableFloat` (`self.Right Sparks`) "Spawn Spacing" _spawn_spacing)
        (`NiagaraComponent.SetVariableFloat` (`self.Right Wing`) "Spawn Spacing" _returnvalue_2)
        (`NiagaraComponent.SetVariableFloat` (`self.Left Sparks`) "Spawn Spacing" _spawn_spacing)
        (`NiagaraComponent.SetVariableFloat` (`self.Left Wing`) "Spawn Spacing" _returnvalue_2)
        (`KismetSystemLibrary.PrintString` (`KismetStringLibrary.Concat_StrStr` (`KismetStringLibrary.Concat_StrStr` (`KismetStringLibrary.Conv_DoubleToString` (`self.spawn rate`)) ", ") (`KismetStringLibrary.Conv_DoubleToString` (`self.spawn spacing`))))))))

(event `set span rate`
  (goto _label))

(event `Key|Five`
  (params (Key :type "Key Structure"))
  (:`Pressed`
    (`/Engine/EditorBlueprintResources/StandardMacros.CompareFloat` (`self.spawn rate`) 260.0
      (:`<`
        (set `self.spawn rate` (`KismetMathLibrary.FMin` (+ (`self.spawn rate`) 10.0) 260.0))
        (set `self.spawn spacing` (/ (`self.spawn spacing`) (`self.spacing multiplier`)))
        (goto _label)))))

(fn `UserConstructionScript`)