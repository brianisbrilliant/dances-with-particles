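; Vive-tracked dancer actor that links a Quinn mesh's IK AnimBP to Live Link transform data and supports recalibration.
; Tick evaluates the Live Link transform and draws it as a debug box.
; Pressing R recalibrates the AnimBP's hands and feet and stores a root offset from the negated tracker location and yaw.
; The logic applying that offset to move the body is disconnected, so the root stays put.
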(event `self.ReceiveBeginPlay`
  (`|ExecutionSequence`
    (:`then_0`
      (bind _asabp_manny_bf_ik (cast `/Game/BrianFolder/ABP_Manny_BF_IK` (`SkeletalMeshComponent.GetAnimInstance` (`self.SKM_QuinnBF_IK`)))) ; get a reference to the animBP, where all the magic happens
      (set `self.AnimBP` _asabp_manny_bf_ik)
      (`KismetSystemLibrary.PrintString` "AnimBP is linked."))
    (:`then_1`
      (`self.EnableInput` (`GameplayStatics.GetPlayerController` 0)) ; so we can press a button to recalibrate
    )
    (:`then_2`
      (`KismetSystemLibrary.DrawDebugBox` (`SceneComponent.K2_GetComponentLocation` (`self.SKM_QuinnBF_IK`)) (30.0 30.0 30.0) (struct :`R` 1.0 :`B` 0.023413 :`A` 1.0) (struct) 60.0 10.0))))

(event `self.ReceiveTick`
  (params (DeltaSeconds :type "Float (single-precision)"))
  (bind _dataresult (`|EvaluateLiveLinkFrameWithSpecificRole` (struct :`Name` "/user/vive_tracker_htcx/role/waist") "/Script/LiveLinkInterface.LiveLinkTransformRole") ; The root of the dancer gets moved around in worldspace
    (:`then`
      (`|ExecutionSequence`
        (:`then_1`
          (bind _transform (break `LiveLinkTransformFrameData` (`.FrameData` (break `LiveLinkTransformBlueprintData` _dataresult))))
          (`KismetSystemLibrary.DrawDebugBox` (.location _transform) (40.0 40.0 40.0) (struct :`R` 0.030457 :`B` 1.0 :`A` 1.0) (.rotation _transform) 0.0 5.0))))))

(event `Key|R`
  (params (Key :type "Key Structure"))
  (:`Pressed`
    (`/Game/BrianFolder/ABP_Manny_BF_IK.Recalibrateeeee` (`self.AnimBP`)) ; This is the Recalibrate function\nFor the hands and feet
    (`self.recalib`) ; This recalibrates root motion
    (`KismetSystemLibrary.PrintString` "Recalibrated" true true (struct :`G` 1.0 :`B` 0.340166 :`A` 1.0))))

(event `recalib`
  (bind _transform (break `LiveLinkTransformFrameData` (`.FrameData` (break `LiveLinkTransformBlueprintData` (stale `self.ReceiveTick` _dataresult)))))
  (bind _output_get (set `self.RootOffset` (`KismetMathLibrary.MakeTransform` (* (.location _transform) -1.0) (`KismetMathLibrary.MakeRotator` 0.0 0.0 (* (.yaw (.rotation _transform)) -1.0)))))
  (`KismetSystemLibrary.DrawDebugBox` (.location _output_get) (50.0 50.0 100.0) (struct :`G` 1.0 :`B` 0.172742 :`A` 1.0) (.rotation _output_get) 10.0 10.0))

(fn `UserConstructionScript`)