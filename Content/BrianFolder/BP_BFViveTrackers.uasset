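; Vive tracker actor that drives Neck, LeftHand and RightHand components from Live Link transforms, with particle wings between neck and hands.
; Tick applies offset and scaling to tracker locations, then aims each wing along neck-to-hand and sets its particle float to that distance.
; Calibrate stores negated tracker locations shortly after BeginPlay or on R, though all three components use the neck's offset.
; Key 0 toggles camera fades; VerticalCheck is empty.
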(event `self.ReceiveTick`
  (params (DeltaSeconds :type "Float (single-precision)"))
  (`self.Debug Lines`)
  (bind _dataresult (`|EvaluateLiveLinkFrameWithSpecificRole` (struct :`Name` "/user/vive_tracker_htcx/role/left_elbow") "/Script/LiveLinkInterface.LiveLinkTransformRole") ; Track Neck
    (:`then`
      (`SceneComponent.K2_SetRelativeTransform` (`self.Neck`) (`KismetMathLibrary.MakeTransform` (* (+ (.location (`.Transform` (break `LiveLinkTransformFrameData` (`.FrameData` (break `LiveLinkTransformBlueprintData` _dataresult))))) (`|GetArrayItem` (`self.Offset`))) (`self.Scaling`))) false false)
      (bind _dataresult_2 (`|EvaluateLiveLinkFrameWithSpecificRole` (struct :`Name` "/user/vive_tracker_htcx/role/camera") "/Script/LiveLinkInterface.LiveLinkTransformRole") ; Track Right Hand
        (:`then`
          (`SceneComponent.K2_SetRelativeTransform` (`self.RightHand`) (`KismetMathLibrary.MakeTransform` (* (+ (.location (`.Transform` (break `LiveLinkTransformFrameData` (`.FrameData` (break `LiveLinkTransformBlueprintData` _dataresult_2))))) (`|GetArrayItem` (`self.Offset`))) (`self.Scaling`))) false false)
          (bind _dataresult_3 (`|EvaluateLiveLinkFrameWithSpecificRole` (struct :`Name` "/user/vive_tracker_htcx/role/chest") "/Script/LiveLinkInterface.LiveLinkTransformRole") ; Track Left Hand
            (:`then`
              (`SceneComponent.K2_SetRelativeTransform` (`self.LeftHand`) (`KismetMathLibrary.MakeTransform` (* (+ (.location (`.Transform` (break `LiveLinkTransformFrameData` (`.FrameData` (break `LiveLinkTransformBlueprintData` _dataresult_3))))) (`|GetArrayItem` (`self.Offset`))) (`self.Scaling`))) false false))))))))

(event `self.ReceiveBeginPlay`
  (bind (_returnvalue_x _returnvalue_y _returnvalue_z) (`KismetMathLibrary.BreakVector` (`SceneComponent.K2_GetComponentLocation` (`self.DefaultSceneRoot`))))
  (`|ExecutionSequence`
    (:`then_0`
      (`self.EnableInput` (`GameplayStatics.GetPlayerController` 0))
      (set `self.StartingHeight` _returnvalue_z))
    (:`then_1`
      (`KismetSystemLibrary.Delay` 0.2)
      (`self.Calibrate`))))

(event `Key|R`
  (params (Key :type "Key Structure"))
  (:`Pressed`
    (`self.Calibrate`)))

(event `Calibrate`
  ;[0 0.6201 1] Brian's calibration based on BF_Vivetracked
  (`KismetArrayLibrary.Array_Set` (`self.Offset`) 0 (* (.location (`.Transform` (break `LiveLinkTransformFrameData` (`.FrameData` (break `LiveLinkTransformBlueprintData` (stale `self.ReceiveTick` _dataresult)))))) -1.0))
  (`KismetArrayLibrary.Array_Set` (`self.Offset`) 1 (* (.location (`.Transform` (break `LiveLinkTransformFrameData` (`.FrameData` (break `LiveLinkTransformBlueprintData` (stale `self.ReceiveTick` _dataresult_2)))))) -1.0))
  (`KismetArrayLibrary.Array_Set` (`self.Offset`) 2 (* (.location (`.Transform` (break `LiveLinkTransformFrameData` (`.FrameData` (break `LiveLinkTransformBlueprintData` (stale `self.ReceiveTick` _dataresult_3)))))) -1.0))
  (`KismetSystemLibrary.PrintString` "." true true (struct :`G` 0.066989 :`B` 1.0 :`A` 1.0) 1.0))

(event `Key|Zero`
  (params (Key :type "Key Structure"))
  (:`Pressed`
    (`self.FlipBlackLevels`)))

(event `FlipBlackLevels`
  (bind _playercameramanager (`PlayerController.PlayerCameraManager` (`GameplayStatics.GetPlayerController` 0)))
  (`/Engine/EditorBlueprintResources/StandardMacros.FlipFlop`
    (:`A`
      (`PlayerCameraManager.StartCameraFade` :`self` _playercameramanager :`ToAlpha` 1.0 :`Duration` 4.0 :`bHoldWhenFinished` true))
    (:`B`
      (`PlayerCameraManager.StartCameraFade` :`self` _playercameramanager :`FromAlpha` 1.0 :`Duration` 4.0 :`bHoldWhenFinished` true))))

(event `look  at hands`
  ;[0.1168 0.08209 1] Getting the Wings to point at the neck
  (`SceneComponent.K2_SetWorldRotation` (`self.Right Wing`) (`KismetMathLibrary.FindLookAtRotation` (`SceneComponent.K2_GetComponentLocation` (`self.Neck`)) (`SceneComponent.K2_GetComponentLocation` (`self.RightHand`))) false false)
  (`SceneComponent.K2_SetWorldRotation` (`self.Left Wing`) (`KismetMathLibrary.FindLookAtRotation` (`SceneComponent.K2_GetComponentLocation` (`self.Neck`)) (`SceneComponent.K2_GetComponentLocation` (`self.LeftHand`))) false false))

(event `Debug Lines`
  ;[1 1 1] Drawing Debug Lines
  (`|ExecutionSequence`
    (:`then_0`
      (`self.look  at hands`))
    (:`then_1`
      ;[0.4479 0 0.2144] Setting the length of the particle emitter equal to the distance between the neck and the hands
      (`NiagaraComponent.SetVariableFloat` (`self.Left Wing`) "float" (`KismetMathLibrary.Vector_Distance` (`SceneComponent.K2_GetComponentLocation` (`self.Neck`)) (`SceneComponent.K2_GetComponentLocation` (`self.LeftHand`)))) ; Set The Distance for the Left Hand to the Neck
      (`NiagaraComponent.SetVariableFloat` (`self.Right Wing`) "float" (`KismetMathLibrary.Vector_Distance` (`SceneComponent.K2_GetComponentLocation` (`self.Neck`)) (`SceneComponent.K2_GetComponentLocation` (`self.RightHand`)))) ; Set the Distance for the Right hand to the Neck
    )
    (:`then_2`
      (`self.VerticalCheck`))))

(event `VerticalCheck`
  ;[1 1 1] make sure the hands don't go in the ground.
)

(fn `UserConstructionScript`)