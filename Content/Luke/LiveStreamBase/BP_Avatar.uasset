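; BP_Avatar is a live-stream avatar whose skeletal mesh runs a Rokoko animation instance, with a stomp effect on the left foot.
; BeginPlay hides the mesh without propagating to its children, then sets the Rokoko instance's Demo value to a demo profile name.
; An overlap on the Foot_l component activates NSStomp for a second before deactivating it, with debug strings printed on overlap begin and end.
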(event `self.ReceiveBeginPlay`
  (`SceneComponent.SetVisibility` (`self.SkeletalMesh`) false false)
  (bind _asrokoko (cast `/Game/Luke/LiveStreamBase/Rokoko` (`SkeletalMeshComponent.GetAnimInstance` (`self.SkeletalMesh`))))
  (set `/Game/Luke/LiveStreamBase/Rokoko.Demo` "DemoProfile" _asrokoko))

(event `self.foot_l.OnComponentBeginOverlap`
  (params (OverlappedComponent :type "PrimitiveComponent Object Reference") (OtherActor :type "Actor Object Reference") (OtherComp :type "PrimitiveComponent Object Reference") (OtherBodyIndex :type Integer) (bFromSweep :type Boolean) (SweepResult :type "HitResult Structure (by ref)"))
  (bind _ns_stomp (`self.NS_Stomp`))
  (`KismetSystemLibrary.PrintString` (`KismetSystemLibrary.GetDisplayName` OtherComp))
  (`ActorComponent.Activate` _ns_stomp false)
  (`KismetSystemLibrary.PrintString` "Activated")
  (`KismetSystemLibrary.Delay` 1.0)
  (`ActorComponent.Deactivate` _ns_stomp)
  (`KismetSystemLibrary.PrintString` "deactivated"))

(event `self.foot_l.OnComponentEndOverlap`
  (params (OverlappedComponent :type "PrimitiveComponent Object Reference") (OtherActor :type "Actor Object Reference") (OtherComp :type "PrimitiveComponent Object Reference") (OtherBodyIndex :type Integer))
  (`KismetSystemLibrary.PrintString` "Hello"))

(fn `UserConstructionScript`)