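; BP_LightControls drives four colored spot lights (red, green, purple, orange) from per-light control settings.
; Every tick it passes each light, its controls and its defaults to a shared SetSpotLight function.
; That function applies visibility and intensity from the controls and lerps the RGB color from default toward control values by the controls' alpha, while color alpha comes straight from the controls.
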(event `self.ReceiveTick`
  (params (DeltaSeconds :type "Float (single-precision)"))
  (`self.Set Spot Light` (`self.SpotLight(Red)`) (`self.LC(Red)`) (`self.LD(Red)`))
  (`self.Set Spot Light` (`self.SpotLight(Green)`) (`self.LC(Green)`) (`self.LD(Green)`))
  (`self.Set Spot Light` (`self.SpotLight(Purple)`) (`self.LC(Purple)`) (`self.LD(Purple)`))
  (`self.Set Spot Light` (`self.SpotLight(Orange)`) (`self.LC(Orange)`) (`self.LD(Orange)`)))

(fn `Set Spot Light`
  (params (`Spot Light` :type "LightComponent Object Reference") (LightControls :type "/Game/Luke/LightControls/S_LightControlVariables Structure") (LightDefaults :type "/Game/Luke/LightControls/S_LightDefaults Structure"))
  (`SceneComponent.SetVisibility` `Spot Light` LightControls_LightOn_18_24106E8F4D403E5C22FA2883FEE49E60 false)
  (`LightComponent.SetIntensity` `Spot Light` LightControls_Intensity_21_8FCA1C8641B26655311BC6B3002C2BCB)
  (`LightComponent.SetLightColor` `Spot Light` (make `LinearColor` (`KismetMathLibrary.Lerp` LightDefaults_LightColorR_8_C548CA36460AEA10FFDBEC88279DFBD9 LightControls_LightColorR_2_1AD725BD422BCE45686074B81C24E42E LightControls_Alpha_24_E6E5F686467607A9BBA4B28D102F602F) (`KismetMathLibrary.Lerp` LightDefaults_LightColorG_9_C6FCCE244C380D5E1A347CB3CD5F1A08 LightControls_LightColorG_8_44F0EAA544932256D26764A4206902BE LightControls_Alpha_24_E6E5F686467607A9BBA4B28D102F602F) (`KismetMathLibrary.Lerp` LightDefaults_LightColorB_10_D70D275F40D9CCBD466055802DB9C880 LightControls_LightColorB_9_BDE542904E56C15E761A27AF538A06F7 LightControls_Alpha_24_E6E5F686467607A9BBA4B28D102F602F) LightControls_LightColorA_10_388A6FB14EB4414CF9CBCE9CC1272A0F) true))

(fn `UserConstructionScript`)