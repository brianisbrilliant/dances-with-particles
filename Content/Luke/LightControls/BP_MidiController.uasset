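; MIDI-driven show controller that turns note presses into stage lighting and camera cues.
; On BeginPlay it binds to a MIDI input device, and a note selector routes notes to directional light rotation, a blackout toggle, spotlight color and zoom cues, or a camera jump.
; Color fades and pawn-position zooms run as frame-delay loops driven by a shared timer with per-cue color durations.
; Control-change and note-off events trigger no effects.
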(event `self.ReceiveBeginPlay`
  ;[0 0 0] Set Midi Controller
  (bind (_outmidiinputdevices _outmidioutputdevices) (`MIDIDeviceManager.FindAllMIDIDeviceInfo`))
  (for _array_element _outmidiinputdevices
    _)
  (for _array_element_2 _outmidioutputdevices
    (if (`self.SetInput`)
      (`KismetSystemLibrary.Delay` 0.2)
      (bind _returnvalue (`MIDIDeviceManager.CreateMIDIDeviceInputController` 1))
      (bind _output_get (set `self.Midi Input` _returnvalue))
      (add `MIDIDeviceInputController.OnMIDINoteOn` _output_get (delegate `MIDI NoteOn`))
      (add `MIDIDeviceInputController.OnMIDINoteOff` _output_get (delegate `MIDI NoteOff`))
      (add `MIDIDeviceInputController.OnMIDIControlChange` _output_get (delegate `MIDI ControlChange`)))))

(event `MIDI NoteOff`
  (params (MIDIDeviceController :type "MIDIDeviceInputController Object Reference") (Timestamp :type Integer) (Channel :type Integer) (Note :type Integer) (Velocity :type Integer))
  ;[0 0 0] Set Midi Controller
)

(event `MIDI ControlChange`
  (params (MIDIDeviceController :type "MIDIDeviceInputController Object Reference") (Timestamp :type Integer) (Channel :type Integer) (Type :type Integer) (Value :type Integer))
  ;[0 0 0] Set Midi Controller
  (bind _knobvalue (`self.ControlChangeSelect` Channel Type Value)))

(event `MIDI NoteOn`
  (params (MIDIDeviceController :type "MIDIDeviceInputController Object Reference") (Timestamp :type Integer) (Channel :type Integer) (Note :type Integer) (Velocity :type Integer))
  (bind _returnvalue (`GameplayStatics.GetPlayerPawn` 0))
  ;[0 0 0] Set Midi Controller
  ;;[0 0 0] NoteOn
  (bind _curmov (`self.NoteOnSelect` Note)
    (:`RaiseLights `
      (bind _outactors (`GameplayStatics.GetAllActorsOfClass` "/Game/Luke/BP_DirectionalLight.BP_DirectionalLight_C"))
      (for _array_element _outactors
        (`/Game/Luke/BP_DirectionalLight.Change Rotation` _array_element)))
    (:`Blackout`
      (`self.Blackout`)
      (bind _asbp_cam (cast `/Game/Luke/LightControls/BP_Cam` _returnvalue))
      (`CameraComponent.SetFieldOfView` (`/Game/Luke/LightControls/BP_Cam.Camera` _asbp_cam) 20.0)
      (`self.K2_SetActorLocation` _returnvalue (0.0 7000.0 400.0) false false))
    (:`LightsAndZoom`
      (set `self.Timer` 0.0)
      (`self.Set Lights` _curmov)
      (if (== _curmov 4)
        (bind _asbp_cam_2 (cast `/Game/Luke/LightControls/BP_Cam` _returnvalue))
        (`CameraComponent.SetFieldOfView` (`/Game/Luke/LightControls/BP_Cam.Camera` _asbp_cam_2) 90.0)
        (`self.ZoomOut` _curmov)
        (else
          (`self.ZoomIn` _curmov))))
    (:`SwitchingWings`
      (bind _asbp_cam_3 (cast `/Game/Luke/LightControls/BP_Cam` (`GameplayStatics.GetPlayerPawn` 0)))
      (`self.K2_SetActorLocationAndRotation` :`self` _asbp_cam_3 :`NewLocation` (3250.0 -225.0 60.0)))))

(event `ZoomIn`
  (params (CurrChange :type Integer))
  (bind _returnvalue (`GameplayStatics.GetPlayerPawn` 0))
  (bind _deltaseconds (`self.DeltaSeconds`))
  (bind (_returnvalue_x _returnvalue_y _returnvalue_z) (`KismetMathLibrary.BreakVector` (`self.K2_GetActorLocation` _returnvalue)))
  (bind _output (`|GetArrayItem` (`self.EndZoom`) CurrChange))
  ;[0 0 0] Zoom In
  (`KismetSystemLibrary.Delay` _deltaseconds :!label _label)
  (bind _timer (`self.SetTimer` _deltaseconds CurrChange))
  (`self.K2_SetActorLocation` _returnvalue (`KismetMathLibrary.VLerp` (`|GetArrayItem` (`self.StartZoom`) CurrChange) _output _timer) false false)
  (if (not (and (>= (.y _output) _returnvalue_y) (>= (.z _output) _returnvalue_z)))
    (goto _label)))

(event `ZoomOut`
  (params (CurrChange :type Integer))
  (bind _returnvalue (`GameplayStatics.GetPlayerPawn` 0))
  (bind _deltaseconds (`self.DeltaSeconds`))
  (bind _finalend (`self.FinalEnd`))
  (bind (_returnvalue_x _returnvalue_y _returnvalue_z) (`KismetMathLibrary.BreakVector` (`self.K2_GetActorLocation` _returnvalue)))
  ;[0 0 0] Zoom Out
  (`KismetSystemLibrary.Delay` _deltaseconds :!label _label_2)
  (bind _timer (`self.SetTimer` _deltaseconds CurrChange))
  (`self.K2_SetActorLocation` _returnvalue (`KismetMathLibrary.VLerp` (`self.FinalStart`) _finalend _timer) false false)
  (if (not (and (>= _returnvalue_y (.y _finalend)) (>= _returnvalue_z (.z _finalend))))
    (goto _label_2)))

(event `self.ReceiveTick`
  (params (DeltaSeconds :type "Float (single-precision)"))
  ;[0 0 0] Tick Check
  (set `self.DeltaSeconds` DeltaSeconds))

(event `Set Lights`
  (params (CurrChange :type Integer))
  (bind _deltaseconds (`self.DeltaSeconds`))
  ;[0 0 0] Set Lights
  (`KismetSystemLibrary.Delay` _deltaseconds :!label _label_3)
  (bind _timer (`self.SetTimer` _deltaseconds CurrChange))
  (bind _outactors (`GameplayStatics.GetAllActorsOfClass` "/Game/Luke/BP_SpotLight.BP_SpotLight_C"))
  (for _array_element _outactors
    (`/Game/Luke/BP_SpotLight.Change Color` _array_element CurrChange _timer)
    (goto _label_3)))

(event `MidiKeyID`
  (params (MIDIDeviceController :type "MIDIDeviceController Object Reference") (Timestamp :type Integer) (EventType :type "EMIDIEventType Enum" :default "Unknown") (Channel :type Integer) (ControlID :type Integer) (Velocity :type Integer) (RawEventType :type Integer))
  ;[0 0 0] Tick Check
  (`/Engine/EditorBlueprintResources/StandardMacros.IsValid` MIDIDeviceController
    (:`Is Valid`
      (if (!= Timestamp 0)
        (`KismetSystemLibrary.PrintText` (`|FormatText` "{Timestamp}; CH {Channel} - {EventType}/ID: {ControlID}, Velocity {Velocity}" (`KismetTextLibrary.Conv_IntToText` Channel) (`KismetTextLibrary.Conv_IntToText` ControlID) (`KismetTextLibrary.Conv_StringToText` (`|GetEnumeratorNameAsString` EventType)) (`KismetTextLibrary.Conv_IntToText` Velocity) (`KismetTextLibrary.Conv_IntToText` RawEventType)))))))

(fn `Blackout`
  (if (`self.Blackout?`)
    (bind _outactors (`GameplayStatics.GetAllActorsOfClass` "/Game/Luke/BP_SpotLight.BP_SpotLight_C"))
    (for _array_element _outactors
      (`LightComponent.SetLightColor` (`/Game/Luke/BP_SpotLight.SpotLight` _array_element) (struct :`R` 0.192708 :`B` 0.001211 :`A` 1.0) true)
      (bind _outactors_2 (`GameplayStatics.GetAllActorsOfClass` "/Game/Luke/BP_DirectionalLight.BP_DirectionalLight_C"))
      (for _array_element_2 _outactors_2
        (`self.K2_SetActorRotation` _array_element_2 (struct :`Pitch` -9.9 :`Yaw` 88.1 :`Roll` -109.2) false)
        (set `self.Blackout?` false)))
    (else
      (bind _outactors_3 (`GameplayStatics.GetAllActorsOfClass` "/Game/Luke/BP_SpotLight.BP_SpotLight_C"))
      (for _array_element_3 _outactors_3
        (`LightComponent.SetLightColor` (`/Game/Luke/BP_SpotLight.SpotLight` _array_element_3) (struct :`A` 1.0) true)
        (bind _outactors_4 (`GameplayStatics.GetAllActorsOfClass` "/Game/Luke/BP_DirectionalLight.BP_DirectionalLight_C"))
        (for _array_element_4 _outactors_4
          (`self.K2_SetActorRotation` _array_element_4 (struct :`Pitch` 50.0) false)
          (set `self.Blackout?` true))))))

(fn `ControlChange`
  (params (Channel :type Integer) (Type :type Integer) (Value :type Integer))
  (`KismetSystemLibrary.PrintText` (`|FormatText` "{Channel}: Type - {Note} - Vel: {Velocity}" Channel Type Value)))

(fn `SetTimer`
  (params (Delta :type "Float (double-precision)") (CurrMov :type Integer))
  (returns (Timer :type "Float (double-precision)"))
  (bind _output_get (set `self.Timer` (+ Delta (`self.Timer`))))
  (return (`KismetMathLibrary.FClamp` (/ _output_get (`|GetArrayItem` (`self.ColorChangeTimes`) CurrMov)))))

(fn `UserConstructionScript`)