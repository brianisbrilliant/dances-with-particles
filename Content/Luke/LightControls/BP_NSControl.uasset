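; BP_NSControl is a Blueprint that drives a Niagara particle effect from its own variables, under a LightControls folder.
; Every Tick it writes particle lifetime, spawn rate, RGB color, minimum and maximum size, and opacity into the component's User parameters.
; Changes to those variables therefore show in the effect on the next frame, with no other logic or construction setup.
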(event `self.ReceiveTick`
  (params (DeltaSeconds :type "Float (single-precision)"))
  (bind _niagaracomponent (`self.NiagaraComponent`))
  (`NiagaraComponent.SetVariableFloat` _niagaracomponent "User.ParticleLifeMax" (`self.ParticleLifeMax`))
  (`NiagaraComponent.SetVariableFloat` _niagaracomponent "User.SpawnRate" (`self.SpawnRate`))
  (`NiagaraComponent.SetVariableVec3` _niagaracomponent "User.Color" (`KismetMathLibrary.MakeVector` (`self.Red`) (`self.Green`) (`self.Blue`)))
  (`NiagaraComponent.SetVariableFloat` _niagaracomponent "User.SizeMin" (`self.MinSize`))
  (`NiagaraComponent.SetVariableFloat` _niagaracomponent "User.SizeMax" (`self.MaxSize`))
  (`NiagaraComponent.SetVariableFloat` _niagaracomponent "User.Opacity" (`self.Opacity`)))

(fn `UserConstructionScript`)