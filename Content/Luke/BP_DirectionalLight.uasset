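; Directional light actor that rotates from a start to an end rotation on BeginPlay, likely as a timed lighting transition.
; A Delay loop paced by the delta seconds stored on Tick lerps the rotation, with duration based on the player BP_Cam's Delay plus an offset, printing each value.
; Once complete, it zeroes that Delay and calls ChangeIntensity on every BP_SpotLight.
; MovementReset is an empty stub.
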(event `self.ReceiveBeginPlay`
  (`self.K2_SetActorRotation` (`self.Start Rotation`))
  (`self.Change Rotation`))

(event `self.ReceiveTick`
  (params (DeltaSeconds :type "Float (single-precision)"))
  (set `self.Delta Seconds` DeltaSeconds))

(event `Change Rotation`
  (bind _delta_seconds (`self.Delta Seconds`))
  (`KismetSystemLibrary.Delay` _delta_seconds :!label _label)
  (bind _asbp_cam (cast `/Game/Luke/LightControls/BP_Cam` (`GameplayStatics.GetPlayerPawn` 0)))
  (bind _output_get (set `self.CurrentTimer` (+ (`self.CurrentTimer`) _delta_seconds)))
  (if (`self.RotationComp`)
    (set `/Game/Luke/LightControls/BP_Cam.Delay` 0 _asbp_cam)
    (bind _outactors (`GameplayStatics.GetAllActorsOfClass` "/Game/Luke/BP_SpotLight.BP_SpotLight_C"))
    (for _array_element _outactors
      (`/Game/Luke/BP_SpotLight.Change Intensity` _array_element))
    (else
      (`self.Rotation Change` (/ _output_get (+ (`/Game/Luke/LightControls/BP_Cam.Delay` _asbp_cam) 5)))
      (goto _label))))

(fn `MovementReset`
  (params (MvmtTime :type "Float (double-precision)")))

(fn `Rotation Change`
  (params (SetTime :type "Float (double-precision)"))
  (bind _returnvalue (`KismetMathLibrary.RLerp` (`self.Start Rotation`) (`self.End Rotation`) SetTime true))
  (`KismetSystemLibrary.PrintString` (`KismetStringLibrary.Conv_RotatorToString` _returnvalue) true true (struct :`R` 0.686685 :`G` 0.124772 :`A` 1.0))
  (`self.K2_SetActorRotation` _returnvalue)
  (set `self.RotationComp` (> SetTime 1.0)))

(fn `UserConstructionScript`)